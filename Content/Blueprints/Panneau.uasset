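; Sign actor (Panneau) whose displayed look is driven by a scalar offset parameter on its materials.
; The construction script applies the configured Décalage value to the parameter named by NomParamètreDécalage.
; On BeginPlay, a one-in-ten random roll replaces that offset with a random entry from an easter egg offset array.
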(event EventBeginPlay
  (bind _décalges_easter_egg (Variables|Default|GetDécalges%20Easter%20egg))
  (if (== (Math|Random|RandomInteger 10) 0)
    (Rendering|Material|SetScalarParameterValueonMaterials (Variables|Default|GetPanneau) (Utilities|String|StringToName (Variables|Default|GetNom%20paramètre%20décalage)) (Utilities|Array|Get(acopy) _décalges_easter_egg (Math|Random|RandomInteger (Utilities|Array|Length _décalges_easter_egg))))))

(fn ConstructionScript
  (Rendering|Material|SetScalarParameterValueonMaterials (Variables|Default|GetPanneau) (Utilities|String|StringToName (Variables|Default|GetNom%20paramètre%20décalage)) (Variables|Default|GetDécalage)))