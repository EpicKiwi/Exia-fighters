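; Game mode that runs a round countdown and returns the game to the main menu when time runs out.
; Tick feeds a one-second Delay, so the Secondes counter drops about once per second without a timer.
; A negative count wraps back to a fixed value, while reaching zero pauses the game and opens the MainMenu level.
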(event EventBeginPlay)

(event EventTick
  (params (DeltaSeconds :type Float%20%28single-precision%29))
  ;[1 1 1] Compteur round
  (Utilities|FlowControl|Delay 1.0)
  (Variables|Default|Setsecondes (- (Variables|Default|Getsecondes) 1))
  (if (< (Math|Conversions|ToFloat(Integer) (Variables|Default|Getsecondes)) 0.0)
    (Variables|Default|Setsecondes 100))
  (if (== (Variables|Default|Getsecondes) 0)
    (Game|SetGamePaused true)
    (Game|OpenLevel(byName) "MainMenu")))

(fn ConstructionScript)